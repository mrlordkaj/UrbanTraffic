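; Urban traffic Blueprint whose visible logic runs a time-of-day cycle for the sun, sky and light system.
; On BeginPlay it sets a Timeline's rate from TimerSpeed and its start point from TimerStart.
; Timeline updates feed UpdateTimeline, which sets sun intensity and pitch, refreshes the sky sphere's sun direction, and passes the current hour to UpdateLightSystem.
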(event `self.ReceiveBeginPlay`
  (`TimelineComponent.SetPlayRate` (`self.Timeline`) (/ (`self.TimerSpeed`) 3600.0))
  (bind (_direction _sun_strength _sun_angle _timer_hour) (`Timeline|Timeline` :`NewTime` (`self.TimerStart`) :!via `SetNewTime`)
    (:`Update`
      (`self.UpdateTimeline` _sun_strength _sun_angle _timer_hour))))

(fn `UpdateTimeline`
  (params (sunStrength :type "Float (double-precision)") (sunAngle :type "Float (double-precision)") (timerHour :type "Float (double-precision)"))
  (`LightComponent.SetIntensity` (`Light.LightComponent` (`self.SunLight`)) sunStrength)
  (`self.K2_SetActorRotation` (`self.SunLight`) (`KismetMathLibrary.MakeRotator` -6.0 (* sunAngle 100.0) 8.0) false)
  (`/Engine/EngineSky/BP_Sky_Sphere.UpdateSunDirection` (`self.SkySphere`))
  (`self.updateLightSystem` timerHour))

(fn `UserConstructionScript`)